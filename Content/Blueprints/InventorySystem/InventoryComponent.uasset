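; Inventory component that records added items and shows them as slots in the inventory UI.
; AddItemToInventory advances a row and column cursor shared by all categories, wrapping at a fixed width, then stores the item class with its add amount.
; It creates an InventorySlot widget and places it at the cursor in the Medic, Resources or Equipment grid, reached through FirstPersonGameMode's display UI.
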(event EventBeginPlay)

(event EventTick
  (params (DeltaSeconds :type Float%20%28single-precision%29)))

(fn AddItemtoInventory
  (params (ItemToAdd :type Item%20Object%20Reference))
  (bind _returnvalue (Game|GetGameMode))
  (bind _itemstructure (Variables|/Game/Blueprints/InventorySystem/InventoryItems/Item.Item_C|GetItemStructure ItemToAdd))
  (bind _itemstructure_2 (Variables|/Game/Blueprints/InventorySystem/InventoryItems/Item.Item_C|GetItemStructure ItemToAdd))
  (bind _freerow (Variables|Default|GetFreeRow))
  (bind _asfirst_person_game_mode (Utilities|Casting|CastToFirstPersonGameMode _returnvalue))
  (bind _displayui (Variables|/Game/Blueprints/FirstPersonGameMode.FirstPersonGameMode_C|GetDisplayUI _asfirst_person_game_mode))
  (bind _inventoryui (Variables|/Game/UserInterface/DisplayUI.DisplayUI_C|GetInventoryUI _displayui))
  (Utilities|FlowControl|Sequence
    (:then_0
      (if (!= (Variables|Default|GetFreeColumn) 15)
        (Math|Integer|IncrementInt (Variables|Default|GetFreeColumn))
        (else
          (Variables|Default|SetFreeColumn 1)
          (Math|Integer|IncrementInt (Variables|Default|GetFreeRow)))))
    (:then_1
      (Utilities|Map|Add (Variables|Default|GetInventoryItems) (Utilities|GetClass ItemToAdd) (.howmanytoadd _itemstructure))
      (switch Utilities|FlowControl|Switch|SwitchonEItemCategories (.itemcategory _itemstructure)
        (:NewEnumerator0
          (bind _returnvalue_2 (UserInterface|CreateWidget "/Game/UserInterface/InventoryUI/InventorySlot.InventorySlot_C" 0 _itemstructure_2))
          (Class|GridPanel|AddChildtoGrid (Variables|/Game/UserInterface/InventoryUI/ItemCategoryUI.ItemCategoryUI_C|GetGridPanel_66 (Variables|/Game/UserInterface/InventoryUI/InventoryUI.InventoryUI_C|GetItemCategoryUI _inventoryui)) _returnvalue_2 _freerow (Variables|Default|GetFreeColumn)))
        (:NewEnumerator1
          (bind _returnvalue_3 (UserInterface|CreateWidget "/Game/UserInterface/InventoryUI/InventorySlot.InventorySlot_C" 0 _itemstructure_2))
          (Class|GridPanel|AddChildtoGrid (Variables|/Game/UserInterface/InventoryUI/ItemCategoryUI.ItemCategoryUI_C|GetGridPanel_66 (Variables|/Game/UserInterface/InventoryUI/InventoryUI.InventoryUI_C|GetItemCategoryUI_1 _inventoryui)) _returnvalue_3 _freerow (Variables|Default|GetFreeColumn)))
        (:NewEnumerator2
          (bind _returnvalue_4 (UserInterface|CreateWidget "/Game/UserInterface/InventoryUI/InventorySlot.InventorySlot_C" 0 _itemstructure_2))
          (Class|GridPanel|AddChildtoGrid (Variables|/Game/UserInterface/InventoryUI/ItemCategoryUI.ItemCategoryUI_C|GetGridPanel_66 (Variables|/Game/UserInterface/InventoryUI/InventoryUI.InventoryUI_C|GetItemCategoryUI_2 _inventoryui)) _returnvalue_4 _freerow (Variables|Default|GetFreeColumn)))))))